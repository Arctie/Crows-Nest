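; BP_collectable is a pickup actor that the player collects with the Interact input while inside its Box trigger.
; Overlap by a BP_playerBase enables the actor's input and shows an EtoCollect prompt widget; leaving disables input, then hides and removes the prompt after a short delay.
; Interacting decrements CollectiblesLeft on BP_GameModeBase, adds a CollectableWidget to the viewport and destroys the actor.
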(event OnComponentBeginOverlap(Box)
  (params (OverlappedComponent :type Primitive%20Component%20Object%20Reference) (OtherActor :type Actor%20Object%20Reference) (OtherComp :type Primitive%20Component%20Object%20Reference) (OtherBodyIndex :type Integer) (bFromSweep :type Boolean) (SweepResult :type Hit%20Result%20Structure%20%28by%20ref%29))
  (Utilities|Casting|CastToBP_playerBase OtherActor)
  (Input|EnableInput (Game|GetPlayerController 0))
  (bind _returnvalue (UserInterface|CreateWidget "/Game/Assets/UserInterface/EtoCollect.EtoCollect_C"))
  (UserInterface|Viewport|AddtoViewport _returnvalue 0))

(event OnComponentEndOverlap(Box)
  (params (OverlappedComponent :type Primitive%20Component%20Object%20Reference) (OtherActor :type Actor%20Object%20Reference) (OtherComp :type Primitive%20Component%20Object%20Reference) (OtherBodyIndex :type Integer))
  (Utilities|Casting|CastToBP_playerBase OtherActor)
  (Input|DisableInput (Game|GetPlayerController 0))
  (Default|HidePickup (stale OnComponentBeginOverlap(Box) _returnvalue))
  (Utilities|FlowControl|Delay 0.3)
  (Widget|RemovefromParent (stale OnComponentBeginOverlap(Box) _returnvalue)))

(event Input|ActionEvents|InputActionInteract
  (params (Key :type Key%20Structure :default "None"))
  (:Pressed
    (bind _asbp_game_mode_base (Utilities|Casting|CastToBP_GameModeBase (Game|GetGameMode)))
    (bind _result (Math|Integer|DecrementInt (Variables|/Game/Blueprints/BP_GameModeBase.BP_GameModeBase_C|GetCollectiblesLeft _asbp_game_mode_base))
      (:%20%20
        (Variables|/Game/Blueprints/BP_GameModeBase.BP_GameModeBase_C|SetCollectiblesLeft _asbp_game_mode_base _result)
        (bind _returnvalue (UserInterface|CreateWidget "/Game/Assets/UserInterface/CollectableWidget.CollectableWidget_C"))
        (UserInterface|Viewport|AddtoViewport _returnvalue 0)
        (Actor|DestroyActor)))))

(fn ConstructionScript)