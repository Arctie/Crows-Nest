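; Base player character Blueprint with jumping, single-axis movement along world X, walk and sprint speeds, and a pause menu toggle.
; BeginPlay caches the default max walk speed, which Walk and Sprint scale by multipliers while held and restore on release.
; The Pause input creates or removes the WB_Pause widget, switching game pause, input mode and mouse cursor visibility to match.
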(event EventBeginPlay
  (Variables|Default|SetdefaultWalkSpeed (Variables|/Script/Engine.CharacterMovementComponent|GetMaxWalkSpeed (Variables|Character|GetCharacterMovement))))

(event Collision|EventActorBeginOverlap
  (params (OtherActor :type Actor%20Object%20Reference)))

(event EventTick
  (params (DeltaSeconds :type Float%20%28single-precision%29)))

(event Input|ActionEvents|InputActionJump
  (params (Key :type Key%20Structure :default "None"))
  ;[0.00472 0.005204 0.01562] Jumping
  (:Pressed
    (Character|Jump))
  (:Released
    (Character|StopJumping)))

(event Input|ActionEvents|InputActionWalk
  (params (Key :type Key%20Structure :default "None"))
  (bind _charactermovement (Variables|Character|GetCharacterMovement))
  (bind _defaultwalkspeed (Variables|Default|GetdefaultWalkSpeed))
  (:Pressed
    (Variables|/Script/Engine.CharacterMovementComponent|SetMaxWalkSpeed _charactermovement (* _defaultwalkspeed (Variables|Default|GetWalkAmount))))
  (:Released
    (Variables|/Script/Engine.CharacterMovementComponent|SetMaxWalkSpeed _charactermovement _defaultwalkspeed)))

(event Input|ActionEvents|InputActionSprint
  (params (Key :type Key%20Structure :default "None"))
  (bind _charactermovement (Variables|Character|GetCharacterMovement))
  (bind _defaultwalkspeed (Variables|Default|GetdefaultWalkSpeed))
  (:Pressed
    (Variables|/Script/Engine.CharacterMovementComponent|SetMaxWalkSpeed _charactermovement (* _defaultwalkspeed (Variables|Default|GetSprintAmount))))
  (:Released
    (Variables|/Script/Engine.CharacterMovementComponent|SetMaxWalkSpeed _charactermovement _defaultwalkspeed)))

(event Input|ActionEvents|InputActionPause
  (params (Key :type Key%20Structure :default "None"))
  (bind _returnvalue (Game|GetPlayerController 0))
  (:Pressed
    (if (Variables|Default|GetPauseOpen)
      (Variables|Default|SetPauseOpen false)
      (Widget|RemovefromParent (Variables|Default|GetPause%20widget))
      (Game|SetGamePaused false)
      (Input|SetInputModeGameOnly _returnvalue)
      (Variables|/Script/Engine.PlayerController|SetbShowMouseCursor (Game|GetPlayerController 0) false)
      (else
        (Variables|Default|SetPauseOpen true)
        (bind _returnvalue_2 (UserInterface|CreateWidget "/Game/Assets/UserInterface/WB_Pause.WB_Pause_C" _returnvalue))
        (bind _output_get (Variables|Default|SetPause%20widget _returnvalue_2))
        (UserInterface|Viewport|AddtoViewport _output_get 0)
        (Game|SetGamePaused true)
        (Input|SetInputModeGameandUI _returnvalue (Variables|Default|GetPause%20widget) "DoNotLock" true)
        (Variables|/Script/Engine.PlayerController|SetbShowMouseCursor (Game|GetPlayerController 0) true)))))

(event Input|AxisEvents|InputAxisMoveRight
  (params (AxisValue :type Float%20%28single-precision%29))
  ;[0.003928 0.02083 0.007275] Movement
  (Pawn|Input|AddMovementInput "1.000000, 0, 0" AxisValue false))

(fn ConstructionScript)